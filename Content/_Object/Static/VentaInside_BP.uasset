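; Interactive vent that the player kicks open from the inner side.
; A trigger box enables kicking and shows the kick progress bar on the player's UI while the player is inside.
; Each click, briefly rate-limited, plays a kick sound and fills the bar, whose percent doubles as the progress state.
; Reaching the threshold unpauses a looping timer that rotates the outer cover until an angle check pauses it.
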(event OnComponentBeginOverlap(Box)
  (params (OverlappedComponent :type Primitive%20Component%20Object%20Reference) (OtherActor :type Actor%20Object%20Reference) (OtherComp :type Primitive%20Component%20Object%20Reference) (OtherBodyIndex :type Integer) (bFromSweep :type Boolean) (SweepResult :type Hit%20Result%20Structure%20%28by%20ref%29))
  ;[1 1 1] IS player near the vent from iner side?
  (if (== OtherActor (Game|GetPlayerCharacter 0))
    (Variables|Default|SetCanOpen true)
    (Widget|SetVisibility (Variables|/Game/_FirstPerson/UI/UI.UI_C|GetKickBar_W (Variables|/Game/_FirstPerson/Blueprints/BP_FirstPersonCharacter.BP_FirstPersonCharacter_C|GetUI%20Ref (Variables|Default|GetCharRef))) "Visible")))

(event OnComponentEndOverlap(Box)
  (params (OverlappedComponent :type Primitive%20Component%20Object%20Reference) (OtherActor :type Actor%20Object%20Reference) (OtherComp :type Primitive%20Component%20Object%20Reference) (OtherBodyIndex :type Integer))
  ;[1 1 1] IS player near the vent from iner side?
  (if (== OtherActor (Game|GetPlayerCharacter 0))
    (Variables|Default|SetCanOpen false)
    (Widget|SetVisibility (Variables|/Game/_FirstPerson/UI/UI.UI_C|GetKickBar_W (Variables|/Game/_FirstPerson/Blueprints/BP_FirstPersonCharacter.BP_FirstPersonCharacter_C|GetUI%20Ref (Variables|Default|GetCharRef))) "Hidden")))

(event Custom|OpenVent
  (bind _ventaoutside (Variables|Default|GetVentaOutside))
  (bind _relativerotation (Variables|/Script/Engine.SceneComponent|GetRelativeRotation _ventaoutside))
  ;[1 1 1] Animation for opening vent
  (Utilities|FlowControl|Sequence
    (:then_0
      (Transformation|AddLocalRotation _ventaoutside (Math|Rotator|MakeRotator 0.0 (- 0.0 3.0) 0.0) false false)
      (if (and (== (.roll _relativerotation) 1.8e+02) (and (>= (.pitch _relativerotation) 0.0) (<= (.pitch _relativerotation) 15.0)))
        (Utilities|Time|PauseTimerbyHandle (Variables|Default|GetOpenVentHnadle))))
    (:then_1
      (Utilities|FlowControl|DoOnce false
        (:Completed
          (Utilities|FlowControl|Delay 0.1)
          (Audio|PlaySound2D "/Game/_Sound/Sounds/Vent/Vent_approach_Cue.Vent_approach_Cue" 1.0 1.0 0.0 0 0))))))

(event EventBeginPlay
  (bind _asbp_first_person_character (Utilities|Casting|CastToBP_FirstPersonCharacter (Game|GetPlayerCharacter 0)))
  (Variables|Default|SetCharRef _asbp_first_person_character)
  (Variables|Default|SetKickAmount 0.25)
  (bind _returnvalue (Utilities|Time|SetTimerbyFunctionName 0 "OpenVent" 0.025 true))
  (bind _output_get (Variables|Default|SetOpenVentHnadle _returnvalue))
  (Utilities|Time|PauseTimerbyHandle _output_get))

(event EventInterefaceObjectClick
  (bind _kickamount (Variables|Default|GetKickAmount))
  (bind _charref (Variables|Default|GetCharRef))
  (bind _ui_ref (Variables|/Game/_FirstPerson/Blueprints/BP_FirstPersonCharacter.BP_FirstPersonCharacter_C|GetUI%20Ref _charref))
  (bind _kickbar_w (Variables|/Game/_FirstPerson/UI/UI.UI_C|GetKickBar_W _ui_ref))
  (bind _progressbar_113 (Variables|/Game/_Object/Static/KickBar_W.KickBar_W_C|GetProgressBar_113 _kickbar_w))
  (bind _percent (Variables|/Script/UMG.ProgressBar|GetPercent _progressbar_113))
  (bind _returnvalue (+ _percent _kickamount))
  (bind _returnvalue_2 (Math|Float|Clamp(Float) _returnvalue))
  ;[1 1 1] Kicking and increasing progress bar amount, if it is full turn off collision and play OpenVent animation (timer)
  (if (Variables|Default|GetCanOpen)
    (Utilities|FlowControl|DoOnce false :!label _label
      (:Completed
        (Progress|SetPercent _progressbar_113 _returnvalue_2)
        (Audio|SpawnSound2D "/Game/_Sound/Sounds/Vent/kickVent_Cue.kickVent_Cue" 0.6 1.0 0.0 0)
        (Utilities|FlowControl|Sequence
          (:then_0
            (if (>= _returnvalue_2 1.0)
              (Utilities|FlowControl|DoOnce false
                (:Completed
                  (Utilities|Time|UnpauseTimerbyHandle (Variables|Default|GetOpenVentHnadle))))))
          (:then_1
            (Utilities|FlowControl|Delay 0.2)
            (goto _label Reset)))))))

(fn ConstructionScript)

(fn InterfaceObjectHold
  (params (Aim%20Movement :type Vector%202D%20Structure)))