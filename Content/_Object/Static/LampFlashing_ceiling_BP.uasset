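; Flickering ceiling lamp actor that briefly flashes its point light at a regular interval.
; BeginPlay starts a looping timer on Flash, with a period randomized once per instance.
; Each Flash sets a random high intensity, waits a short random delay, then drops the light to a dim level.
; Material swaps on the Neonka component are present but disconnected, so only the light changes.
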(event Custom|Flash
  (Rendering|Components|Light|SetIntensity (Variables|Default|GetPointLight) (Math|Random|RandomFloatinRange 2e+02 2e+03))
  (Utilities|FlowControl|Delay (Math|Random|RandomFloatinRange 0.05 0.1))
  (Rendering|Components|Light|SetIntensity (Variables|Default|GetPointLight) 1.0))

(event EventBeginPlay
  (Utilities|Time|SetTimerbyFunctionName 0 "Flash" (Math|Random|RandomFloatinRange 1.0 2.5) true))

(fn ConstructionScript)