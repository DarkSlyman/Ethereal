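; SafeTimer_BP is an actor that generates a random safe code in clock format and displays it on a text render.
; On BeginPlay, GetSafeNumbers fills the SafeCode array with an hour-range and two minute-range values, shown colon-separated.
; It aims to avoid adjacent duplicates by clearing and retrying on a match, but each check uses a separate random roll from the value added.
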(event EventBeginPlay
  (bind _safecode (Variables|Default|GetSafeCode))
  (CallFunction|GetSafeNumbers)
  (Rendering|Components|TextRender|SetText (Variables|Default|GetTextRender) (Utilities|Text|ToText(String) (Utilities|String|Append (Utilities|String|ToString(Text) (Utilities|Text|ToText(Integer) (Utilities|Array|Get(acopy) _safecode) false true 2 2)) ":" (Utilities|String|ToString(Text) (Utilities|Text|ToText(Integer) (Utilities|Array|Get(acopy) _safecode 1) false true 2 2)) ":" (Utilities|String|ToString(Text) (Utilities|Text|ToText(Integer) (Utilities|Array|Get(acopy) _safecode 2) false true 2 2))))))

(fn ConstructionScript)

(fn GetSafeNumbers
  (bind _returnvalue (Math|Random|RandomIntegerinRange 0 59))
  (bind _returnvalue_2 (Math|Random|RandomIntegerinRange 0 59))
  ;[1 1 1] Make sure you dont have two same numbers going after each other
  (Utilities|Array|Add (Variables|Default|GetSafeCode) (Math|Random|RandomIntegerinRange 0 23) :!label _label)
  (if (== _returnvalue (Utilities|Array|Get(acopy) (Variables|Default|GetSafeCode)))
    (Utilities|Array|Clear (Variables|Default|GetSafeCode) :!label _label_2)
    (goto _label)
    (else
      (Utilities|Array|Add (Variables|Default|GetSafeCode) _returnvalue)
      (if (== _returnvalue_2 (Utilities|Array|Get(acopy) (Variables|Default|GetSafeCode) 1))
        (goto _label_2)
        (else
          (Utilities|Array|Add (Variables|Default|GetSafeCode) _returnvalue_2))))))