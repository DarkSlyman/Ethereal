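; Interactable vent cover that opens either by removing its four screws or by kicking it from inside.
; The object-hold interface picks the aimed screw, and holding with a screwdriver ("srobovak") as the current item backs it out until it is destroyed.
; Inside the trigger box, which shows the kick bar UI, holding triggers cooldown-spaced kicks, opening on the third.
; Opening disables actor collision and swings the cover via a timeline.
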(event OnComponentBeginOverlap(Box)
  (params (OverlappedComponent :type Primitive%20Component%20Object%20Reference) (OtherActor :type Actor%20Object%20Reference) (OtherComp :type Primitive%20Component%20Object%20Reference) (OtherBodyIndex :type Integer) (bFromSweep :type Boolean) (SweepResult :type Hit%20Result%20Structure%20%28by%20ref%29))
  ;[1 1 1] IS player near the vent from iner side?
  (if (== OtherActor (Game|GetPlayerCharacter 0))
    (Variables|Default|SetCanOpen true)
    (Widget|SetVisibility (Variables|/Game/_FirstPerson/UI/UI.UI_C|GetKickBar_W (Variables|/Game/_FirstPerson/Blueprints/BP_FirstPersonCharacter.BP_FirstPersonCharacter_C|GetUI%20Ref (Variables|Default|GetCharRef))) "Visible")))

(event OnComponentEndOverlap(Box)
  (params (OverlappedComponent :type Primitive%20Component%20Object%20Reference) (OtherActor :type Actor%20Object%20Reference) (OtherComp :type Primitive%20Component%20Object%20Reference) (OtherBodyIndex :type Integer))
  ;[1 1 1] IS player near the vent from iner side?
  (if (== OtherActor (Game|GetPlayerCharacter 0))
    (Variables|Default|SetCanOpen false)
    (Widget|SetVisibility (Variables|/Game/_FirstPerson/UI/UI.UI_C|GetKickBar_W (Variables|/Game/_FirstPerson/Blueprints/BP_FirstPersonCharacter.BP_FirstPersonCharacter_C|GetUI%20Ref (Variables|Default|GetCharRef))) "Hidden")))

(event Custom|Holding
  (bind _charref (Variables|Default|GetCharRef))
  (bind _screwindex (Variables|Default|GetScrewIndex))
  (bind _screws (Variables|Default|GetScrews))
  (bind _numberofscrews (Variables|Default|GetNumberOfScrews))
  (bind _output (Utilities|Array|Get(acopy) _screws _screwindex))
  ;[1 1 1] Check if you have screwdriver
  (if (Utilities|String|Contains (Utilities|GetDisplayName (Utilities|Array|Get(acopy) (Variables|/Game/_FirstPerson/Blueprints/BP_FirstPersonCharacter.BP_FirstPersonCharacter_C|GetInv _charref) (Variables|/Game/_FirstPerson/Blueprints/BP_FirstPersonCharacter.BP_FirstPersonCharacter_C|GetCurrent%20Item _charref))) "srobovak")
    ;[1 1 1] Animation for screws
    (Utilities|IsValid _output
      (:Is%20Valid
        (if (<= (.x (Variables|/Script/Engine.SceneComponent|GetRelativeLocation _output)) 8.0)
          (Transformation|AddRelativeLocation _output "0.200000,0.000000,0.000000" false false)
          (Transformation|AddRelativeRotation _output "0.000000,0.000000,15.000000" false false)
          (else
            (Utilities|FlowControl|Delay 0.2)
            (Math|Integer|DecrementInt _numberofscrews
              (:%20%20
                (if (<= _numberofscrews 0)
                  (CallFunction|OpenVent))
                (Components|DestroyComponent _output)))))))))

(event Custom|OpenVent
  (bind _ventaoutside (Variables|Default|GetVentaOutside))
  (bind _returnvalue (Transformation|GetWorldRotation _ventaoutside))
  ;[1 1 1] Animation for opening vent
  (Utilities|FlowControl|DoOnce false
    (:Completed
      (Utilities|FlowControl|Delay 0.1)
      (Collision|SetActorEnableCollision false)
      (bind _newtrack_0 (Timeline|Timeline Play)
        (:Update
          (Transformation|SetWorldRotation _ventaoutside (Math|Rotator|MakeRotator (.roll _returnvalue) (- (.pitch _returnvalue) (* _newtrack_0 3.0)) (.yaw _returnvalue)) false false))))))

(event Custom|Kicking
  ;[1 1 1] Kicking bar
  (Utilities|FlowControl|DoOnce false :!label _label
    (:Completed
      (if (== (Variables|Default|GetKickAmount) 1.0)
        (if (== (Variables|Default|GetKickAmount2) 1.0)
          (Variables|Default|SetKickAmount3 1.0)
          (Utilities|FlowControl|Delay 0.1)
          (CallFunction|OpenVent)
          (else
            (Variables|Default|SetKickAmount2 1.0)
            (Variables|/Game/_FirstPerson/Blueprints/BP_FirstPersonCharacter.BP_FirstPersonCharacter_C|SetInteracting (Variables|Default|GetCharRef) false)
            (Utilities|FlowControl|Delay 1.0 :!label _label_2)
            (goto _label Reset)))
        (else
          (Variables|Default|SetKickAmount 1.0)
          (Variables|/Game/_FirstPerson/Blueprints/BP_FirstPersonCharacter.BP_FirstPersonCharacter_C|SetInteracting (Variables|Default|GetCharRef) false)
          (goto _label_2))))))

(event EventBeginPlay
  (bind _asbp_first_person_character (Utilities|Casting|CastToBP_FirstPersonCharacter (Game|GetPlayerCharacter 0)))
  (Variables|Default|SetCharRef _asbp_first_person_character)
  (Variables|Default|SetScrews (Utilities|Array|MakeArray (Variables|Default|GetScrewRT) (Variables|Default|GetScrewLT) (Variables|Default|GetScrewRB) (Variables|Default|GetScrewLB)))
  (Variables|Default|SetNumberOfScrews 4)
  (Variables|Default|SetKickAmount 0.0)
  (Variables|Default|SetKickAmount2 0.0)
  (Variables|Default|SetKickAmount3 0.0))

(fn ConstructionScript)

(fn InterfaceObjectHold
  (params (Aim%20Movement :type Vector%202D%20Structure))
  (if (Variables|Default|GetCanOpen)
    (CallFunction|Kicking)
    (return (Transformation|GetWorldLocation (Variables|Default|GetVentaCenter)))
    (else
      (switch string (Utilities|GetObjectName (Variables|/Game/_FirstPerson/Blueprints/BP_FirstPersonCharacter.BP_FirstPersonCharacter_C|GetAimedActorComponent (Variables|Default|GetCharRef)))
        (:Default
          (return (Transformation|GetWorldLocation (Variables|Default|GetVentaCenter))))
        (:CapsuleRT
          (Variables|Default|SetScrewIndex 0)
          (CallFunction|Holding)
          (return (Transformation|GetWorldLocation (Variables|Default|GetCapsuleRT))))
        (:CapsuleLT
          (Variables|Default|SetScrewIndex 1)
          (CallFunction|Holding)
          (return (Transformation|GetWorldLocation (Variables|Default|GetCapsuleLT))))
        (:CapsuleRB
          (Variables|Default|SetScrewIndex 2)
          (CallFunction|Holding)
          (return (Transformation|GetWorldLocation (Variables|Default|GetCapsuleRB))))
        (:CapsuleLB
          (Variables|Default|SetScrewIndex 3)
          (CallFunction|Holding)
          (return (Transformation|GetWorldLocation (Variables|Default|GetCapsuleLB))))))))