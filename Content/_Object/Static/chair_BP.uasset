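; Chair actor whose static mesh spins continuously while bobbing up and down in an endless loop.
; On BeginPlay, a fast looping timer fires a custom event that adds a fixed yaw rotation to the mesh in stepped increments.
; Two timelines alternate, one playing forward and the other in reverse, each driving the mesh's relative Z location and restarting the other when finished.
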(event Custom|CustomEvent_0
  (Transformation|AddWorldRotation (Variables|Default|GetStaticMesh) "0,10.000000, 0" false false))

(event EventBeginPlay
  (Utilities|Time|SetTimerbyEvent (delegate Custom|CustomEvent_0) 0.05 true)
  (bind _newtrack_0 (Timeline|Timeline PlayFromStart)
    (:Update
      (Transformation|SetRelativeLocation (Variables|Default|GetStaticMesh) (Math|Vector|MakeVector 0.0 0.0 (* _newtrack_0 2e+02)) false false))
    (:Finished
      (bind _newtrack_0_2 (Timeline|Timeline_0 ReverseFromEnd)
        (:Update
          (Transformation|SetRelativeLocation (Variables|Default|GetStaticMesh) (Math|Vector|MakeVector 0.0 0.0 (* _newtrack_0_2 2e+02)) false false))
        (:Finished
          (Timeline|Timeline PlayFromStart))))))

(fn ConstructionScript)