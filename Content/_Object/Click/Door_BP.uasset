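; Interactive door that the player swings open or shut by holding and dragging, unless it is locked.
; InterfaceObjectHold flips horizontal drag when the player is outside NormalSide, triggers the RotateSwitch timeline through Moving, and returns a focus socket location.
; OpenAI and CloseAI provide separate timeline swings with sound, but their in-file callers (enemy overlap, click toggle) are disconnected.
; TooltipTextik passes tooltip text to the player character.
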(event OnComponentBeginOverlap(Box)
  (params (OverlappedComponent :type Primitive%20Component%20Object%20Reference) (OtherActor :type Actor%20Object%20Reference) (OtherComp :type Primitive%20Component%20Object%20Reference) (OtherBodyIndex :type Integer) (bFromSweep :type Boolean) (SweepResult :type Hit%20Result%20Structure%20%28by%20ref%29)))

(event OnComponentEndOverlap(Box)
  (params (OverlappedComponent :type Primitive%20Component%20Object%20Reference) (OtherActor :type Actor%20Object%20Reference) (OtherComp :type Primitive%20Component%20Object%20Reference) (OtherBodyIndex :type Integer)))

(event Custom|OpenAI
  ;[1 1 1] Otavaranie a zatvaranie, nastavenie či sú dvere opened/closed
  (Audio|PlaySoundatLocation "/Game/_Sound/Sounds/doors/Door_Opening.Door_Opening" (Transformation|GetActorLocation) "0, 0, 0" 1.0 1.0 0.0 0 0 0 0)
  (bind _newtrack_0 (Timeline|Timeline_0 Play)
    (:Update
      (Transformation|SetRelativeRotation (Variables|Default|GetDoor) (Math|Rotator|MakeRotator 0.0 0.0 (* _newtrack_0 9e+01)) false false))
    (:Finished
      (Variables|Default|SetOpened? true)
      (bind _newtrack_0_2 (Timeline|Timeline_1 SetNewTime)
        (:Update
          (Transformation|SetRelativeRotation (Variables|Default|GetDoor) (Math|Rotator|MakeRotator 0.0 0.0 (* _newtrack_0_2 9e+01)) false false))
        (:Finished
          (Variables|Default|SetOpened? false)
          (Timeline|Timeline_0 SetNewTime))))))

(event Custom|Moving
  (if (not (Variables|Default|GetLocked?))
    (if (Variables|Default|GetSwitch%20position)
      (bind _newtrack_0 (Timeline|rotate%20switch Reverse)
        (:Update
          (Transformation|SetRelativeRotation (Variables|Default|GetDoor) (Math|Rotator|MakeRotator 0.0 0.0 _newtrack_0) false false))
        (:Finished
          (Variables|Default|SetSwitch%20position (not (Variables|Default|GetSwitch%20position)))))
      (else
        (Timeline|rotate%20switch Play)))))

(event Custom|CloseAI
  ;[1 1 1] Otavaranie a zatvaranie, nastavenie či sú dvere opened/closed
  (Utilities|FlowControl|Sequence
    (:then_0
      (bind _newtrack_0 (Timeline|Timeline_1 Reverse)
        (:Update
          (Transformation|SetRelativeRotation (Variables|Default|GetDoor) (Math|Rotator|MakeRotator 0.0 0.0 (* _newtrack_0 9e+01)) false false))
        (:Finished
          (Variables|Default|SetOpened? false)
          (bind _newtrack_0_2 (Timeline|Timeline_0 SetNewTime)
            (:Update
              (Transformation|SetRelativeRotation (Variables|Default|GetDoor) (Math|Rotator|MakeRotator 0.0 0.0 (* _newtrack_0_2 9e+01)) false false))
            (:Finished
              (Variables|Default|SetOpened? true)
              (Timeline|Timeline_1 SetNewTime))))))
    (:then_1
      (Utilities|FlowControl|Delay 0.8)
      (Audio|PlaySoundatLocation "/Game/_Sound/Sounds/doors/Door_Closing_Cue.Door_Closing_Cue" (Transformation|GetActorLocation) "0, 0, 0" 1.0 1.0 0.0 0 0 0 0))))

(event EventBeginPlay
  ;[1 1 1] Begin play
  (Variables|Default|SetOpened? false)
  (bind _returnvalue (Actor|GetActorOfClass "/Game/_FirstPerson/Blueprints/BP_FirstPersonCharacter.BP_FirstPersonCharacter_C"))
  (Variables|Default|Setchar _returnvalue))

(event EventTick
  (params (DeltaSeconds :type Float%20%28single-precision%29)))

(event EventInterefaceObjectClick)

(event EventTooltipTextik
  (Variables|/Game/_FirstPerson/Blueprints/BP_FirstPersonCharacter.BP_FirstPersonCharacter_C|SetTooltipTextToDisplay (Variables|Default|Getchar) (Variables|Default|GetTooltipToSet)))

(fn ConstructionScript)

(fn InterfaceObjectHold
  (params (Aim%20Movement :type Vector%202D%20Structure))
  (bind _x (Math|Vector2D|BreakVector2D Aim%20Movement))
  (if (Collision|IsOverlappingActor (Variables|Default|GetNormalSide) (Game|GetPlayerCharacter 0) :!class /Script/Engine.PrimitiveComponent)
    (Variables|Default|SetX%20vector _x)
    (else
      (Variables|Default|SetX%20vector (* _x -1.0))))
  (if (or (and (not (Variables|Default|GetSwitch%20position)) (>= (Variables|Default|GetX%20vector) 0.5)) (and (<= (Variables|Default|GetX%20vector) -0.5) (Variables|Default|GetSwitch%20position))) ; Determine whether to move the switch based on drag direction
    (CallFunction|Moving))
  (return (Transformation|GetSocketLocation (Variables|Default|GetScene) "Focus Target")))