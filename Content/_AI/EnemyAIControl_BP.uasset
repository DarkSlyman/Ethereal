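; AI controller for patrolling enemies that runs Enemy_BT and feeds its blackboard.
; BeginPlay seeds the patrol path looping flag, direction and a randomized wait time.
; Perception updates map stimuli by array index: the first sets CanSeePlayer, the second briefly clears IsInvestigating? before setting it and TargetLocation after a delay.
; The Sense function and NewMacro_0 duplicate this logic, the former only partially, and the event graph uses neither.
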(event OnPerceptionUpdated(AIPerception)
  (params (UpdatedActors :type Array%20of%20Actor%20Object%20References))
  (for _array_element UpdatedActors
    (bind (_info _returnvalue) (Class|AIPerceptionComponent|GetActorsPerception (Variables|Default|GetAIPerception) _array_element))
    (for (_array_element_2 _array_index) (.lastsensedstimuli _info)
      (Variables|Default|SetSense_L _array_element_2)
      (switch int _array_index
        (:0
          (AI|Components|Blackboard|SetValueasBool (AI|GetBlackboard 0) (Utilities|Name|MakeLiteralName "CanSeePlayer") (.bsuccessfullysensed (Variables|Default|GetSense_L))))
        (:1
          (AI|Components|Blackboard|SetValueasBool (AI|GetBlackboard 0) (Utilities|Name|MakeLiteralName "IsInvestigating?") false)
          (Utilities|FlowControl|Delay 0.2)
          (AI|Components|Blackboard|SetValueasBool (AI|GetBlackboard 0) (Utilities|Name|MakeLiteralName "IsInvestigating?") (.bsuccessfullysensed (Variables|Default|GetSense_L)))
          (AI|Components|Blackboard|SetValueasVector (AI|GetBlackboard 0) (Utilities|Name|MakeLiteralName "TargetLocation") (.stimuluslocation (Variables|Default|GetSense_L))))))
    (Variables|Default|SetPlayerSensed _returnvalue)))

(event EventBeginPlay
  (AI|RunBehaviorTree "/Game/_AI/Enemy_BT.Enemy_BT")
  (Utilities|FlowControl|Delay 0.2)
  (bind _asenemy_bp (Utilities|Casting|CastToEnemy_BP (Pawn|GetControlledPawn)))
  (Variables|Default|SetEnemyRef _asenemy_bp)
  (AI|Components|Blackboard|SetValueasBool (AI|GetBlackboard 0) (Utilities|Name|MakeLiteralName "PathLooping") (Variables|/Game/_AI/PatrolPath_BP.PatrolPath_BP_C|GetIsLooping (Variables|/Game/_AI/Enemy_BP.Enemy_BP_C|GetPatrolPath (Variables|Default|GetEnemyRef))))
  (Class|BlackboardComponent|SetValueasInt (AI|GetBlackboard 0) (Utilities|Name|MakeLiteralName "Direction") 1)
  (AI|Components|Blackboard|SetValueasFloat (AI|GetBlackboard 0) (Utilities|Name|MakeLiteralName "WaitTime") (+ (Variables|WaitTime|GetWaitTime) (Math|Random|RandomFloatinRange 0.0 (Variables|WaitTime|GetFluctiation)))))

(fn ConstructionScript)

(fn Sense
  (params (Array :type Array%20of%20AI%20Stimulus%20Structures))
  (for (_array_element _array_index) Array
    (LocalVariables|SetSense_L _array_element)
    (switch int _array_index
      (:0
        (AI|Components|Blackboard|SetValueasBool (AI|GetBlackboard 0) (Utilities|Name|MakeLiteralName "CanSeePlayer") (.bsuccessfullysensed (LocalVariables|GetSense_L))))
      (:1
        (AI|Components|Blackboard|SetValueasBool (AI|GetBlackboard 0) (Utilities|Name|MakeLiteralName "IsInvestigating?") false)))))