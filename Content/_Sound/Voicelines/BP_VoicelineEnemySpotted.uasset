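; Overlap trigger actor that plays the enemy-spotted voiceline once, when the first-person character enters it carrying an item with "Card" in its name.
; On overlap it searches the character's inventory display names, with a DoOnce gating the response.
; It then plays the 2D sound, reveals the enemy text in the game menu and runs a timeline animating the opacity of the HUD's writing image and text.
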(event EventBeginPlay
  (|CallParentFunction) ; This node is disabled and will not be called.\nDrag off pins to build functionality.
)

(event Collision|EventActorBeginOverlap
  (params (OtherActor :type Actor%20Object%20Reference))
  (|CallParentFunction OtherActor)
  (bind _asbp_first_person_character (Utilities|Casting|CastToBP_FirstPersonCharacter OtherActor))
  (for _array_element (Variables|/Game/_FirstPerson/Blueprints/BP_FirstPersonCharacter.BP_FirstPersonCharacter_C|GetInv _asbp_first_person_character)
    (if (Utilities|String|Contains (Utilities|GetDisplayName _array_element) "Card")
      (Utilities|FlowControl|DoOnce false
        (:Completed
          (Utilities|FlowControl|Sequence
            (:then_0
              (Audio|PlaySound2D "/Game/_Sound/Sounds/Pero_2.Pero_2" 1.3 1.1 0.0 0 0)
              (Widget|SetVisibility (Variables|/Game/_Menu/GameMenu.GameMenu_C|GetEnemyText (Variables|/Game/_FirstPerson/Blueprints/BP_FirstPersonCharacter.BP_FirstPersonCharacter_C|GetGameMenu _asbp_first_person_character)) "Visible"))
            (:then_1
              (bind _newtrack_0 (Timeline|Timeline PlayFromStart)
                (:Update
                  (Widget|SetRenderOpacity (Variables|/Game/_FirstPerson/UI/UI.UI_C|GetWrittingImage (Variables|/Game/_FirstPerson/Blueprints/BP_FirstPersonCharacter.BP_FirstPersonCharacter_C|GetUI%20Ref _asbp_first_person_character)) _newtrack_0)
                  (Widget|SetRenderOpacity (Variables|/Game/_FirstPerson/UI/UI.UI_C|GetWrittingText (Variables|/Game/_FirstPerson/Blueprints/BP_FirstPersonCharacter.BP_FirstPersonCharacter_C|GetUI%20Ref _asbp_first_person_character)) _newtrack_0))))))))))

(event EventTick
  (params (DeltaSeconds :type Float%20%28single-precision%29))
  (|CallParentFunction DeltaSeconds) ; This node is disabled and will not be called.\nDrag off pins to build functionality.
)

(fn ConstructionScript
  (|CallParentFunction))