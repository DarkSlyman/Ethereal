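; Trigger actor that plays a 2D voiceline about a keycard when the first-person character overlaps it without carrying one.
; On the first character overlap, it scans the Inv array for a display name containing "card", skipping everything if Rozpravam is already set.
; If none is found, it plays the line and holds the character's Rozpravam flag for a fixed delay to block overlap.
; The DoOnce is spent even when no line plays.
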(event EventBeginPlay
  (|CallParentFunction) ; This node is disabled and will not be called.\nDrag off pins to build functionality.
)

(event Collision|EventActorBeginOverlap
  (params (OtherActor :type Actor%20Object%20Reference))
  (|CallParentFunction OtherActor)
  (bind _asbp_first_person_character (Utilities|Casting|CastToBP_FirstPersonCharacter OtherActor))
  (Utilities|FlowControl|DoOnce false
    (:Completed
      (if (not (Variables|/Game/_FirstPerson/Blueprints/BP_FirstPersonCharacter.BP_FirstPersonCharacter_C|GetRozpravam? _asbp_first_person_character))
        (bind _array_element (Utilities|Array|ForEachLoopwithBreak (Variables|/Game/_FirstPerson/Blueprints/BP_FirstPersonCharacter.BP_FirstPersonCharacter_C|GetInv _asbp_first_person_character) :!label _label)
          (:LoopBody
            (if (Utilities|String|Contains (Utilities|GetDisplayName _array_element) "card")
              (Variables|Default|SetKeycard true)
              (goto _label Break)))
          (:Completed
            (if (not (Variables|Default|GetKeycard))
              (Audio|PlaySound2D "/Game/_Sound/Voicelines/Sounds/AKeyCardForThe_Cue.AKeyCardForThe_Cue" 2.0 1.0 0.0 0 0)
              (Variables|/Game/_FirstPerson/Blueprints/BP_FirstPersonCharacter.BP_FirstPersonCharacter_C|SetRozpravam? _asbp_first_person_character true)
              (Utilities|FlowControl|Delay 3.0)
              (Variables|/Game/_FirstPerson/Blueprints/BP_FirstPersonCharacter.BP_FirstPersonCharacter_C|SetRozpravam? _asbp_first_person_character false))))))))

(event EventTick
  (params (DeltaSeconds :type Float%20%28single-precision%29))
  (|CallParentFunction DeltaSeconds) ; This node is disabled and will not be called.\nDrag off pins to build functionality.
)

(fn ConstructionScript
  (|CallParentFunction))